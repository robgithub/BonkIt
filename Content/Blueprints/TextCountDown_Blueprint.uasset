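; Countdown timer Blueprint that displays the remaining time on a TextRender component.
; StartCountdown stores the calling object and restores the initial value saved at BeginPlay.
; While counting, Tick uses a Delay to subtract time in tenth-second steps and refresh the text.
; Dropping below zero clamps the value and calls TimedOut on the stored object, repeating each step until StopCountdown clears the counting flag.
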(event `self.ReceiveBeginPlay`
  (set `self.fltSaveCountDown` (`self.fltCountDownValue`)))

(event `self.ReceiveTick`
  (params (DeltaSeconds :type "Float (single-precision)"))
  (if (`self.blnCountingDown`)
    (`KismetSystemLibrary.Delay` 0.1)
    (set `self.fltCountDownValue` (- (`self.fltCountDownValue`) 0.1))
    (if (not (>= (`self.fltCountDownValue`) 0.0))
      (set `self.fltCountDownValue` 0.0)
      (`/Game/Blueprints/StartCube_Blueprint.TimedOut` (`self.localStartObject`)))
    (`TextRenderComponent.K2_SetText` (`self.TextRender`) (`KismetTextLibrary.Conv_DoubleToText` (`self.fltCountDownValue`) "HalfToEven" false true 2 324 2 2))))

(event `StartCountdown`
  (params (StartObejct :type "/Game/Blueprints/StartCube_Blueprint Object Reference"))
  (set `self.localStartObject` StartObejct)
  (set `self.blnCountingDown` true)
  (set `self.fltCountDownValue` (`self.fltSaveCountDown`)))

(event `StopCountdown`
  (set `self.blnCountingDown` false))

(fn `UserConstructionScript`)