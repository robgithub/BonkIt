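; A three-colour VR button for a timed reaction game, struck with a motion controller.
; A start object activates it via evtBtnActivate, turning it red for the level's speed delay.
; A controller overlap while active turns it green; a timeout counts as a miss, each with its own sound.
; After a lit delay it reports hit or miss to the start object, with blue as the idle colour.
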(event `self.StaticMeshComponent.OnComponentBeginOverlap`
  (params (OverlappedComponent :type "PrimitiveComponent Object Reference") (OtherActor :type "Actor Object Reference") (OtherComp :type "PrimitiveComponent Object Reference") (OtherBodyIndex :type Integer) (bFromSweep :type Boolean) (SweepResult :type "HitResult Structure (by ref)"))
  (bind _asbp_motion_controller (cast `/Game/VirtualRealityBP/Blueprints/BP_MotionController` OtherActor))
  (`self.isCurrentMotionController` _asbp_motion_controller)
  (if (and (not (`self.btnHit`)) (`self.btnActivated`))
    (`PrimitiveComponent.SetMaterial` (`self.StaticMeshComponent`) 0 "/Game/Meshes/Green.Green")
    (set `self.btnHit` true)
    (`AudioComponent.Play` (`self.bonkit_hit_Cue`) 0.0)
    (`KismetSystemLibrary.Delay` (`self.btnLitDelay`))
    (set `self.btnActivated` false)
    (set `self.btnHit` false)
    (`self.resetButtonColour`)
    (`/Game/Blueprints/StartCube_Blueprint.evtButtonHit` (`self.localStartObject`))))

(event `self.StaticMeshComponent.OnComponentEndOverlap`
  (params (OverlappedComponent :type "PrimitiveComponent Object Reference") (OtherActor :type "Actor Object Reference") (OtherComp :type "PrimitiveComponent Object Reference") (OtherBodyIndex :type Integer))
  (bind _asbp_motion_controller (cast `/Game/VirtualRealityBP/Blueprints/BP_MotionController` OtherActor))
  (`self.isCurrentMotionController` _asbp_motion_controller)
  (set `self.blnTrackingMotionController` false))

(event `evtResetState`
  (set `self.btnActivated` false)
  (set `self.btnHit` false)
  (`self.resetButtonColour`))

(event `evtBtnActivate`
  (params (StartObject :type "/Game/Blueprints/StartCube_Blueprint Object Reference") (levelSpeed :type "Float (double-precision)"))
  (if (not (and (not (`self.btnHit`)) (`self.btnActivated`)))
    (set `self.btnActivated` true)
    (set `self.btnHit` false)
    (bind _output_get (set `self.localStartObject` StartObject))
    (`PrimitiveComponent.SetMaterial` (`self.StaticMeshComponent`) 0 "/Game/Meshes/Red.Red")
    (`KismetSystemLibrary.Delay` levelSpeed)
    (if (`self.btnActivated`)
      (if (not (`self.btnHit`))
        (`self.resetButtonColour`)
        (set `self.btnHit` true)
        (`AudioComponent.Play` (`self.bonkit_miss_Cue`) 0.0)
        (`KismetSystemLibrary.Delay` (`self.btnLitDelay`))
        (set `self.btnActivated` false)
        (`/Game/Blueprints/StartCube_Blueprint.evtButtonMissed` _output_get)))))

(fn `isCurrentMotionController`
  (params (mc :type "/Game/VirtualRealityBP/Blueprints/BP_MotionController Object Reference"))
  (returns (isCurrentMC :type Boolean))
  (if (not (`self.blnTrackingMotionController`))
    (set `self.MC_tracking` mc)
    (set `self.blnTrackingMotionController` true)
    (return (== (`self.MC_tracking`) mc))))

(fn `resetButtonColour`
  (`PrimitiveComponent.SetMaterial` (`self.StaticMeshComponent`) 0 "/Game/Meshes/Blue.Blue") ; reseting colour after sucessfully hit
)

(fn `UserConstructionScript`)