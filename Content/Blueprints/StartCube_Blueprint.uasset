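; Start cube that runs a whack-a-button VR mini-game, started by a motion controller touching it.
; Starting hides the force field, zeroes both scores, starts the countdown and activates a random button.
; Button hit and miss events update their counter, lower the level speed value to a floor, then clear all buttons and activate another at random.
; Timeout ends the round with a game-over cue and restores the force field after a delay.
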(event `self.ReceiveBeginPlay`
  (set `self.fltSavedLevelSpeed` (`self.fltLevelSpeed`)))

(event `self.StaticMeshComponent.OnComponentBeginOverlap`
  (params (OverlappedComponent :type "PrimitiveComponent Object Reference") (OtherActor :type "Actor Object Reference") (OtherComp :type "PrimitiveComponent Object Reference") (OtherBodyIndex :type Integer) (bFromSweep :type Boolean) (SweepResult :type "HitResult Structure (by ref)"))
  (bind _asbp_motion_controller (cast `/Game/VirtualRealityBP/Blueprints/BP_MotionController` OtherActor))
  (`/Game/VirtualRealityBP/Blueprints/BP_MotionController.RumbleController` _asbp_motion_controller 0.1)
  (if (not (`self.blnLevelStarted`))
    (set `self.blnLevelStarted` true)
    (`TextRenderComponent.K2_SetText` (`self.TextRenderStart`) (`KismetTextLibrary.Conv_StringToText` (`self.txtGameInProgress`)))
    (`self.SetActorHiddenInGame` (`self.actorForceField`) true)
    (set `self.intHitCount` 0)
    (`self.SetScoreText` (`self.intHitCount`) (`self.actorHitCount`))
    (set `self.intMissCount` 0)
    (`self.SetScoreText` (`self.intMissCount`) (`self.actorMissCount`))
    (`/Game/Blueprints/TextCountDown_Blueprint.StartCountdown` (`self.actorCountDownText`) self)
    (`self.ActiveNextRandomButton` self)
    (`AudioComponent.Play` (`self.bonkit_voice_bonkit_Cue`) 0.0)))

(event `evtButtonHit`
  (bind _fltminlevelspeed (`self.fltMinLevelSpeed`))
  (set `self.btnInPlay` false)
  (if (`self.blnLevelStarted`)
    (`/Engine/EditorBlueprintResources/StandardMacros.IncrementInt` (`self.intHitCount`)
      (:`  `
        (`self.SetScoreText` (`self.intHitCount`) (`self.actorHitCount`))
        (bind _output_get (set `self.fltLevelSpeed` (- (`self.fltLevelSpeed`) 0.3) :!label _label))
        (if (< _output_get _fltminlevelspeed)
          (set `self.fltLevelSpeed` _fltminlevelspeed))
        (`self.ActiveNextRandomButton` self)))))

(event `evtButtonMissed`
  (set `self.btnInPlay` false)
  (if (`self.blnLevelStarted`)
    (`/Engine/EditorBlueprintResources/StandardMacros.IncrementInt` (`self.intMissCount`)
      (:`  `
        (`self.SetScoreText` (`self.intMissCount`) (`self.actorMissCount`))
        (goto _label)))))

(event `TimedOut`
  (if (`self.blnLevelStarted`)
    (set `self.blnLevelStarted` false)
    (`TextRenderComponent.K2_SetText` (`self.TextRenderStart`) (`KismetTextLibrary.Conv_StringToText` (`self.txtGameStart`)))
    (`AudioComponent.Play` (`self.bonkit_gameover_Cue`) 0.0)
    (`KismetSystemLibrary.Delay` 10.0)
    (`self.SetActorHiddenInGame` (`self.actorForceField`) false)))

(fn `ActivateButton`
  (params (Button :type "Object Object Reference") (StartObject :type "/Game/Blueprints/StartCube_Blueprint Object Reference"))
  (bind _asbutton_three_colour_blueprint (cast `/Game/Blueprints/button_three_colour_Blueprint` Button))
  (if (not (`self.btnInPlay`))
    (`|ExecutionSequence`
      (:`then_0`
        (set `self.btnInPlay` true))
      (:`then_1`
        (`/Game/Blueprints/button_three_colour_Blueprint.evtBtnActivate` _asbutton_three_colour_blueprint StartObject (`self.fltLevelSpeed`))
        (`AudioComponent.Play` (`self.bonkit_wah_Cue`) 0.0)))))

(fn `ActiveNextRandomButton`
  (params (StartObject :type "/Game/Blueprints/StartCube_Blueprint Object Reference"))
  (bind _outactors (`GameplayStatics.GetAllActorsOfClass` "/Game/Blueprints/button_three_colour_Blueprint.button_three_colour_Blueprint_C"))
  (`self.ClearButtonsInPlay` _outactors)
  (bind _button (`self.GetRandomButton` _outactors))
  (`self.ActivateButton` _button StartObject))

(fn `ClearButtonsInPlay`
  (params (Buttons :type "Array of /Game/Blueprints/button_three_colour_Blueprint Object Reference"))
  (for _array_element Buttons
    (bind _asbutton_three_colour_blueprint (cast `/Game/Blueprints/button_three_colour_Blueprint` _array_element))
    (`/Game/Blueprints/button_three_colour_Blueprint.evtREsetState` _asbutton_three_colour_blueprint)))

(fn `GetRandomButton`
  (params (Buttons :type "Array of /Game/Blueprints/button_three_colour_Blueprint Object Reference"))
  (returns (Button :type "/Game/Blueprints/button_three_colour_Blueprint Object Reference"))
  (bind _result (`/Engine/EditorBlueprintResources/StandardMacros.DecrementInt` (`KismetArrayLibrary.Array_Length` Buttons)) ; 0 based array
    (:`  `
      (return (`|GetArrayItem` Buttons (`KismetMathLibrary.RandomIntegerInRange` 0 _result))))))

(fn `SetScoreText`
  (params (Score :type Integer) (TextActor :type "TextRenderActor Object Reference"))
  (`TextRenderComponent.K2_SetText` (`TextRenderActor.TextRender` TextActor) (`KismetTextLibrary.Conv_IntToText` Score false true 3)))

(fn `UserConstructionScript`)